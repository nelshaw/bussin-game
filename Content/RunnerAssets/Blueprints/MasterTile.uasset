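; Endless-runner floor tile that populates three lanes and extends the track as the player runs through it.
; On BeginPlay, SpawnObstacle re-rolls per check to place a box, car, coin or student at each lane arrow, left to right; an empty lane ends the chain.
; Player overlap with its Box asks the GameMode to spawn the next tile, adds multiplied score, then destroys this tile after a short delay.
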(event `self.ReceiveBeginPlay`
  (`self.SpawnObstacle`))

(event `self.Box.OnComponentBeginOverlap`
  (params (OverlappedComponent :type "PrimitiveComponent Object Reference") (OtherActor :type "Actor Object Reference") (OtherComp :type "PrimitiveComponent Object Reference") (OtherBodyIndex :type Integer) (bFromSweep :type Boolean) (SweepResult :type "HitResult Structure (by ref)"))
  (cast `/Game/ThirdPersonBP/Blueprints/ThirdPersonCharacter` OtherActor)
  (bind _asthird_person_game_mode (cast `/Game/ThirdPersonBP/Blueprints/ThirdPersonGameMode` (`GameplayStatics.GetGameMode`)))
  (`/Game/ThirdPersonBP/Blueprints/ThirdPersonGameMode.SpawnTile` _asthird_person_game_mode)
  (bind _asthird_person_game_mode_2 (cast `/Game/ThirdPersonBP/Blueprints/ThirdPersonGameMode` (`GameplayStatics.GetGameMode`)))
  (set `/Game/ThirdPersonBP/Blueprints/ThirdPersonGameMode.CurrentScore` (+ (* 1 (`/Game/ThirdPersonBP/Blueprints/ThirdPersonGameMode.ScoreMultiplier` _asthird_person_game_mode_2)) (`/Game/ThirdPersonBP/Blueprints/ThirdPersonGameMode.CurrentScore` _asthird_person_game_mode_2)) _asthird_person_game_mode_2)
  (bind _asthird_person_character (cast `/Game/ThirdPersonBP/Blueprints/ThirdPersonCharacter` (`GameplayStatics.GetPlayerCharacter` 0)))
  (`KismetSystemLibrary.Delay` 0.5)
  (`self.K2_DestroyActor`))

(fn `SpawnObstacle`
  (bind _returnvalue (`KismetMathLibrary.RandomFloatInRange` 0.0 1.0))
  (bind _returnvalue_2 (`KismetMathLibrary.RandomFloatInRange` 0.0 1.0))
  (bind _returnvalue_3 (`KismetMathLibrary.RandomFloatInRange` 0.0 1.0))
  (bind _returnvalue_4 (`SceneComponent.K2_GetComponentToWorld` (`self.LeftArrow`)))
  (bind _returnvalue_5 (`SceneComponent.K2_GetComponentToWorld` (`self.MiddleArrow`)))
  (bind _returnvalue_6 (`SceneComponent.K2_GetComponentToWorld` (`self.RightArrow`)))
  ;[1 1 1] Left Lane Logic
  (if (`KismetMathLibrary.InRange_FloatFloat` _returnvalue_2 0.0 0.2)
    (`|SpawnActorFromClass` "/Game/RunnerAssets/Blueprints/Obstacle_SmallBox.Obstacle_SmallBox_C" _returnvalue_4 "Undefined" "OverrideRootScale" null null)
    ;[1 1 1] Middle Lane Logic
    (if (`KismetMathLibrary.InRange_FloatFloat` _returnvalue_3 0.0 0.2) :!label _label
      (`|SpawnActorFromClass` "/Game/RunnerAssets/Blueprints/Obstacle_SmallBox.Obstacle_SmallBox_C" _returnvalue_5 "Undefined" "OverrideRootScale" null null)
      ;[1 1 1] Right Lane Logic
      (if (`KismetMathLibrary.InRange_FloatFloat` _returnvalue 0.0 0.2) :!label _label_2
        (`|SpawnActorFromClass` "/Game/RunnerAssets/Blueprints/Obstacle_SmallBox.Obstacle_SmallBox_C" _returnvalue_6 "Undefined" "OverrideRootScale" null null)
        (elif (`KismetMathLibrary.InRange_FloatFloat` _returnvalue 0.2 0.3)
          (`|SpawnActorFromClass` "/Game/RunnerAssets/Blueprints/Obstacle_small_car.Obstacle_small_car_C" _returnvalue_6 "Undefined" "OverrideRootScale" null null)
          (elif (`KismetMathLibrary.InRange_FloatFloat` _returnvalue 0.4 0.8)
            (`|SpawnActorFromClass` "/Game/RunnerAssets/Blueprints/Coin.Coin_C" _returnvalue_6 "Undefined" "OverrideRootScale" null null)
            (elif (`KismetMathLibrary.InRange_FloatFloat` _returnvalue 0.8)
              (`|SpawnActorFromClass` "/Game/RunnerAssets/Blueprints/Student.Student_C" _returnvalue_6 "Undefined" "OverrideRootScale" null null)))))
      (elif (`KismetMathLibrary.InRange_FloatFloat` _returnvalue_3 0.2 0.3)
        (`|SpawnActorFromClass` "/Game/RunnerAssets/Blueprints/Obstacle_small_car.Obstacle_small_car_C" _returnvalue_5 "Undefined" "OverrideRootScale" null null)
        (goto _label_2)
        (elif (`KismetMathLibrary.InRange_FloatFloat` _returnvalue_3 0.4 0.8)
          (`|SpawnActorFromClass` "/Game/RunnerAssets/Blueprints/Coin.Coin_C" _returnvalue_5 "Undefined" "OverrideRootScale" null null)
          (goto _label_2)
          (elif (`KismetMathLibrary.InRange_FloatFloat` _returnvalue_3 0.8)
            (`|SpawnActorFromClass` "/Game/RunnerAssets/Blueprints/Student.Student_C" _returnvalue_5 "Undefined" "OverrideRootScale" null null)
            (goto _label_2)))))
    (elif (`KismetMathLibrary.InRange_FloatFloat` _returnvalue_2 0.2 0.3)
      (`|SpawnActorFromClass` "/Game/RunnerAssets/Blueprints/Obstacle_small_car.Obstacle_small_car_C" _returnvalue_4 "Undefined" "OverrideRootScale" null null)
      (goto _label)
      (elif (`KismetMathLibrary.InRange_FloatFloat` _returnvalue_2 0.4 0.8)
        (`|SpawnActorFromClass` "/Game/RunnerAssets/Blueprints/Coin.Coin_C" _returnvalue_4 "Undefined" "OverrideRootScale" null null)
        (goto _label)
        (elif (`KismetMathLibrary.InRange_FloatFloat` _returnvalue_2 0.8)
          (`|SpawnActorFromClass` "/Game/RunnerAssets/Blueprints/Student.Student_C" _returnvalue_4 "Undefined" "OverrideRootScale" null null)
          (goto _label))))))

(fn `UserConstructionScript`)